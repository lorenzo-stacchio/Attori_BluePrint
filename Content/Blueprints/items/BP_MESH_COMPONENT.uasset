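; BP_MESH_COMPONENT is an actor that moves continuously along a looping, oscillating path around the world origin, raised by a fixed height.
; Tick accumulates delta time into T and TC, then sets an absolute location using sine of T for X and Z and cosine of TC for Y.
; AMPLITUDE scales all three axes.
; BeginPlay, the disabled overlap event and the construction script hold no logic.
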(event `self.ReceiveBeginPlay`)

(event `self.ReceiveTick`
  (params (DeltaSeconds :type "Float (single-precision)"))
  (bind _amplitude (`self.AMPLITUDE`))
  (bind _output_get (set `self.T` (+ DeltaSeconds (`self.T`))))
  (bind _output_get_2 (set `self.TC` (+ DeltaSeconds (`self.TC`))))
  (bind _returnvalue (* (`KismetMathLibrary.Sin` _output_get) _amplitude))
  (`self.K2_SetActorLocation` (`KismetMathLibrary.MakeVector` _returnvalue (* (`KismetMathLibrary.Cos` _output_get_2) _amplitude) (+ _returnvalue 200.0))))

(fn `UserConstructionScript`)